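; GhostSpawner is a placed actor that spawns a ghost character of a configurable class at its own transform.
; After an initial delay on BeginPlay it spawns the ghost and assigns it the spawner's GhostColour.
; It binds to the ghost's OnDestroyed event, so each destroyed ghost is replaced after a respawn delay, keeping the cycle going.
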(event Custom|Spawn
  ;[1 1 1] Spawn a ghost
  (bind _returnvalue (Game|SpawnActorfromClass (Variables|Default|GetGhostCharacterClass) (Transformation|GetActorTransform) "AdjustIfPossibleButAlwaysSpawn" 0 0))
  ;[1 1 1] Set the ghost's colour
  (bind _asghost_character (Utilities|Casting|CastToGhostCharacter _returnvalue))
  (Variables|/Game/Blueprints/GhostCharacter.GhostCharacter_C|SetGhostColour _asghost_character (Variables|Default|GetGhostColour))
  ;[1 1 1] When the ghost is destroyed, make it respawn after a delay
  (Game|AssignOnDestroyed _asghost_character (delegate Custom|OnDestroyed_Event_0)))

(event Custom|OnDestroyed_Event_0
  (params (DestroyedActor :type Actor%20Object%20Reference))
  ;[1 1 1] When the ghost is destroyed, make it respawn after a delay
  (Utilities|FlowControl|Delay (Variables|Default|GetDelayOnRespawn))
  (CallFunction|Spawn))

(event EventBeginPlay
  ;[1 1 1] Wait, and then spawn a ghost
  (Utilities|FlowControl|Delay (Variables|Default|GetDelayOnGameStart))
  (CallFunction|Spawn))

(fn ConstructionScript)