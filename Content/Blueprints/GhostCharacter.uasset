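; GhostCharacter is a ghost enemy in a Pac-Man-style game that kills the player on hit, or is destroyed instead while a power pill is active.
; It reads the power pill state from ThirdPersonGameMode.
; The construction script creates a dynamic material, and Tick polls that state to switch its colour and wobble between normal and powered-pill looks.
; PowerPillStatusChanged is an empty stub.
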(event EventTick
  (params (DeltaSeconds :type Float%20%28single-precision%29))
  (bind _material (Variables|Default|GetMaterial))
  ;[1 1 1] Set material properties
  (bind _powerpillactive (Utilities|GetPowerPillActive))
  (Rendering|Material|SetVectorParameterValue _material "Colour" (select _powerpillactive "(R=0.506356,G=0.479167,B=1.000000,A=1.000000)" (Variables|Default|GetGhostColour)) :!class /Script/Engine.MaterialInstanceDynamic)
  (Rendering|Material|SetScalarParameterValue _material "Wobble" (select _powerpillactive 2e+01 0.1) :!class /Script/Engine.MaterialInstanceDynamic))

(event Collision|EventHit
  (params (MyComp :type Primitive%20Component%20Object%20Reference) (Other :type Actor%20Object%20Reference) (OtherComp :type Primitive%20Component%20Object%20Reference) (bSelfMoved :type Boolean) (HitLocation :type Vector :default "0, 0, 0") (HitNormal :type Vector :default "0, 0, 0") (NormalImpulse :type Vector :default "0, 0, 0") (Hit :type Hit%20Result%20Structure%20%28by%20ref%29))
  ;[1 1 1] Check if hit by player
  (bind _asplayer_character (Utilities|Casting|CastToPlayerCharacter Other))
  ;[1 1 1] Branch on power pill state
  (bind _powerpillactive (Utilities|GetPowerPillActive))
  (if _powerpillactive
    ;[1 1 1] Power pill active -> destroy ghost
    (Actor|DestroyActor)
    (else
      ;[1 1 1] Power pill not active -> destroy player
      (Actor|DestroyActor _asplayer_character))))

(fn ConstructionScript
  ;[1 1 1] Create and store dynamic material
  (bind _returnvalue (Rendering|Material|CreateDynamicMaterialInstance (Variables|Default|GetStaticMesh) 0 "/Game/Geometry/Meshes/GhostMaterial.GhostMaterial" "None" :!class /Script/Engine.PrimitiveComponent))
  (Variables|Default|SetMaterial _returnvalue))

(fn PowerPillStatusChanged
  (params (PowerPillActive :type Boolean)))